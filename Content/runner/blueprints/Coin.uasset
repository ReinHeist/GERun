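; Collectible coin for a runner game that adds to the Runnermode coin count when the run_character touches it.
; Pickup plays a sound, destroys the coin and calls UpdateCoins on the character.
; The coin also destroys itself when it overlaps an ObstaclesWall or PowerUp_Magnet.
; A separate Sphere overlap starts the magnet pull if IsMagnetAct is set, using the Slide timeline to interpolate the coin toward the player.
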(event OnComponentBeginOverlap(Sphere)
  (params (OverlappedComponent :type Primitive%20Component%20Object%20Reference) (OtherActor :type Actor%20Object%20Reference) (OtherComp :type Primitive%20Component%20Object%20Reference) (OtherBodyIndex :type Integer) (bFromSweep :type Boolean) (SweepResult :type Hit%20Result%20Structure%20%28by%20ref%29))
  (bind _asrun_character (Utilities|Casting|CastTorun_character OtherActor))
  (if (Variables|/Game/runner/blueprints/run_character.run_character_C|GetIsMagnetAct _asrun_character)
    (bind _slide (Timeline|Slide PlayFromStart)
      (:Update
        (Transformation|SetActorLocation (+ _slide (Math|Interpolation|VInterpTo (.Location (Math|Transform|BreakTransform (Transformation|GetActorTransform))) (Transformation|GetActorLocation (Game|GetPlayerCharacter 0)) (Utilities|Time|GetWorldDeltaSeconds) 2e+01)) false false)))))

(event OnComponentBeginOverlap(coin)
  (params (OverlappedComponent :type Primitive%20Component%20Object%20Reference) (OtherActor :type Actor%20Object%20Reference) (OtherComp :type Primitive%20Component%20Object%20Reference) (OtherBodyIndex :type Integer) (bFromSweep :type Boolean) (SweepResult :type Hit%20Result%20Structure%20%28by%20ref%29))
  (Utilities|FlowControl|Sequence
    (:then_0
      (bind _asrun_character (Utilities|Casting|CastTorun_character OtherActor))
      (bind _asrunnermode (Utilities|Casting|CastToRunnermode (Game|GetGameMode)))
      (Math|Integer|IncrementInt (Variables|/Game/runner/blueprints/Runnermode.Runnermode_C|GetCoins _asrunnermode)
        (:%20%20
          (Audio|PlaySound2D "/Game/runner/Meshes/350874__cabled_mess__coin_c_08.350874__cabled_mess__coin_c_08" 1.0 1.0 0.0 0 0)
          (Actor|DestroyActor)
          (Default|UpdateCoins _asrun_character))))
    (:then_1
      (Utilities|Casting|CastToObstaclesWall OtherActor)
      (Actor|DestroyActor))
    (:then_2
      (Utilities|Casting|CastToPowerUp_Magnet OtherActor)
      (Actor|DestroyActor))))

(fn ConstructionScript)