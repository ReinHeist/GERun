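; Floor tile for an endless runner that populates itself with obstacles, coins and an occasional power-up.
; The construction script builds arrow spawn points along each lane, then shuffles them to place child actors, adding a power-up when the game mode's FloorCount exceeds a threshold, then resetting it.
; Box overlap asks Runnermode to extend the floor, slightly raises clamped player speed and adds multiplier-based points.
; GetAttachPoint exposes the Arrow's world transform.
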(event OnComponentBeginOverlap(Box)
  (params (OverlappedComponent :type Primitive%20Component%20Object%20Reference) (OtherActor :type Actor%20Object%20Reference) (OtherComp :type Primitive%20Component%20Object%20Reference) (OtherBodyIndex :type Integer) (bFromSweep :type Boolean) (SweepResult :type Hit%20Result%20Structure%20%28by%20ref%29))
  ;[1 1 1] extend floor
  (bind _asrunnermode (Utilities|Casting|CastToRunnermode (Game|GetGameMode)))
  (Default|ExtendFloor _asrunnermode)
  ;[1 1 1] change speed
  (bind _asrun_character (Utilities|Casting|CastTorun_character (Game|GetPlayerCharacter 0)))
  (Variables|/Script/Engine.CharacterMovementComponent|SetMaxWalkSpeed (Variables|/Script/Engine.Character|GetCharacterMovement _asrun_character) (Math|Float|Clamp(Float) (* (Variables|/Script/Engine.CharacterMovementComponent|GetMaxWalkSpeed (Variables|/Script/Engine.Character|GetCharacterMovement _asrun_character)) 1.001) 7e+02 1.5e+03))
  ;[1 1 1] Set Current Score
  (bind _asrunnermode_2 (Utilities|Casting|CastToRunnermode (Game|GetGameMode)))
  (Variables|/Game/runner/blueprints/Runnermode.Runnermode_C|SetCurrent%20Points _asrunnermode_2 (+ (* (Variables|/Game/runner/blueprints/Runnermode.Runnermode_C|GetMultiPoints _asrunnermode_2) 1) (Variables|/Game/runner/blueprints/Runnermode.Runnermode_C|GetCurrent%20Points _asrunnermode_2))))

(event EventBeginPlay)

(event Collision|EventActorBeginOverlap
  (params (OtherActor :type Actor%20Object%20Reference)))

(event EventTick
  (params (DeltaSeconds :type Float%20%28single-precision%29)))

(fn ConstructionScript
  (CallFunction|Setupspawnpoints)
  (CallFunction|SpawnObstacles)
  (CallFunction|CoinSpawnPoints)
  (CallFunction|SpawnCoins)
  (CallFunction|PowerUpSpawnPoints)
  (CallFunction|SpawnPowerUp))

(fn GetAttachPoint
  (return (Transformation|GetWorldTransform (Variables|Default|GetArrow))))

(fn Setupspawnpoints
  (for _array_element (Variables|Default|GetLanePosition)
    (for _index (range 0 1)
      (bind _returnvalue (AddComponent|AddArrowComponent false (Math|Transform|MakeTransform (Math|Vector|MakeVector (* _index 6.5e+02) _array_element 0.0))))
      (Utilities|Array|Add (Variables|Default|Getspawn%20points) (Transformation|GetWorldTransform _returnvalue)))))

(fn SpawnObstacles
  (bind _output_get (LocalVariables|Setrandom%20spawn%20point (Variables|Default|Getspawn%20points)))
  (Utilities|Array|Shuffle _output_get)
  (for _index (range 0 (Math|Random|RandomIntegerinRange 0 2))
    (switch int (Math|Random|RandomIntegerinRange 0 1)
      (:0
        (AddComponent|AddChildActorComponent false (Math|Transform|MakeRelativeTransform (Utilities|Array|Get(acopy) (LocalVariables|Getrandom%20spawn%20point) _index) (Transformation|GetActorTransform))))
      (:1
        (AddComponent|AddChildActorComponent false (Math|Transform|MakeRelativeTransform (Utilities|Array|Get(acopy) (LocalVariables|Getrandom%20spawn%20point) _index) (Transformation|GetActorTransform)))))))

(fn CoinSpawnPoints
  (for _array_element (Variables|Default|GetLanePosition)
    (for _index (range 0 6)
      (bind _returnvalue (AddComponent|AddArrowComponent false (Math|Transform|MakeTransform (Math|Vector|MakeVector (* _index 75.0) _array_element 0.0))))
      (Variables|/Script/Engine.ArrowComponent|SetArrowColor _returnvalue "")
      (Utilities|Array|Add (Variables|Default|GetCSpawnPoint) (Transformation|GetWorldTransform _returnvalue)))))

(fn SpawnCoins
  (bind _output_get (LocalVariables|Setrandom%20spawn%20point (Variables|Default|GetCSpawnPoint)))
  (Utilities|Array|Shuffle _output_get)
  (for _index (range 0 (Math|Random|RandomIntegerinRange 3 6))
    (switch int 0
      (:0
        (AddComponent|AddChildActorComponent false (Math|Transform|MakeRelativeTransform (Utilities|Array|Get(acopy) (LocalVariables|Getrandom%20spawn%20point) _index) (Transformation|GetActorTransform)))))))

(fn PowerUpSpawnPoints
  (for _array_element (Variables|Default|GetLanePosition)
    (for _index (range 1 2)
      (bind _returnvalue (AddComponent|AddArrowComponent false (Math|Transform|MakeTransform (Math|Vector|MakeVector (* _index 2.5e+02) _array_element 0.0))))
      (Variables|/Script/Engine.ArrowComponent|SetArrowColor _returnvalue "")
      (Utilities|Array|Add (Variables|Default|GetPSpawnPoints) (Transformation|GetWorldTransform _returnvalue)))))

(fn SpawnPowerUp
  (bind _asrunnermode (Utilities|Casting|CastToRunnermode (Game|GetGameMode)))
  (if (> (Variables|/Game/runner/blueprints/Runnermode.Runnermode_C|GetFloor%20Count _asrunnermode) 5)
    (bind _output_get (LocalVariables|Setrandom%20spawn%20point (Variables|Default|GetPSpawnPoints)))
    (Utilities|Array|Shuffle _output_get)
    (switch int 0
      (:0
        (AddComponent|AddChildActorComponent false (Math|Transform|MakeRelativeTransform (Utilities|Array|Get(acopy) (LocalVariables|Getrandom%20spawn%20point)) (Transformation|GetActorTransform)))
        (Variables|/Game/runner/blueprints/Runnermode.Runnermode_C|SetFloor%20Count _asrunnermode 0)))))