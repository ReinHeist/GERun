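; Magnet power-up pickup for a runner game that switches on the player character's magnet flag for about ten seconds.
; On player overlap it plays a coin sound, hides itself and, unless a magnet is already active, starts a per-second Runnermode countdown.
; A parallel delay clears the flag and destroys the actor, which stays alive hidden until then.
; Overlapping an ObstaclesWall destroys the pickup.
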(event Collision|EventActorBeginOverlap
  (params (OtherActor :type Actor%20Object%20Reference))
  (Utilities|FlowControl|Sequence
    (:then_0
      (bind _asrun_character (Utilities|Casting|CastTorun_character OtherActor))
      (bind _asrunnermode (Utilities|Casting|CastToRunnermode (Game|GetGameMode)))
      (Audio|PlaySound2D "/Game/runner/Meshes/350874__cabled_mess__coin_c_08.350874__cabled_mess__coin_c_08" 1.0 1.0 0.0 0 0)
      (Rendering|SetActorHiddenInGame true)
      (if (not (Variables|/Game/runner/blueprints/run_character.run_character_C|GetIsMagnetAct _asrun_character))
        (Variables|/Game/runner/blueprints/run_character.run_character_C|SetIsMagnetAct _asrun_character true)
        (Variables|/Game/runner/blueprints/Runnermode.Runnermode_C|SetMagnetTimer _asrunnermode 11)
        (Development|PrintString "Magnet ACtive")
        (Utilities|FlowControl|Sequence
          (:then_0
            (Utilities|ForLoopwithDelay 0 10 1.0
              (:LoopBody
                (bind _result (Math|Float|DecrementFloat (Math|Conversions|ToFloat(Integer) (Variables|/Game/runner/blueprints/Runnermode.Runnermode_C|GetMagnetTimer _asrunnermode)))
                  (:%20%20
                    (bind _output_get (Variables|/Game/runner/blueprints/Runnermode.Runnermode_C|SetMagnetTimer _asrunnermode (Math|Float|Truncate (Math|Float|Max(Float) _result 0.0))))
                    (Development|PrintString (Utilities|String|ToString(Integer) _output_get) true true "(R=0.247224,G=1.000000,B=0.163749,A=1.000000)"))))))
          (:then_1
            (Utilities|FlowControl|Delay 10.2)
            (bind _asrun_character_2 (Utilities|Casting|CastTorun_character (Game|GetPlayerCharacter 0)))
            (Variables|/Game/runner/blueprints/run_character.run_character_C|SetIsMagnetAct _asrun_character_2 false)
            (Development|PrintString "Magnet inACtive")
            (Actor|DestroyActor)))))
    (:then_1
      (Utilities|Casting|CastToObstaclesWall OtherActor)
      (Actor|DestroyActor))))

(fn ConstructionScript)