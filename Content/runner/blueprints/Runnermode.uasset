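; Runner game mode for an endless runner that spawns and recycles the floor tiles and buildings along the track.
; BeginPlay builds the initial floor and building chains, reloading the saved coin total from the CoinValue slot inside the floor loop.
; Each spawned piece's attach point becomes the next spawn transform.
; ExtendFloor and ExtendBuildings append a piece and destroy the oldest once their array exceeds its limit.
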(event EventBeginPlay
  (Utilities|FlowControl|Sequence
    (:then_0
      (for _index (range 0 (- (Variables|Default|GetNumber%20of%20Tyles) 1))
        (CallFunction|AddFloor)
        (bind _returnvalue (SaveGame|LoadGamefromSlot "CoinValue"))
        (bind _asrunner_save_game (Utilities|Casting|CastToRunner_SaveGame _returnvalue))
        (Variables|Default|SetCoins (Variables|/Game/runner/blueprints/Runner_SaveGame.Runner_SaveGame_C|GetCoinValue _asrunner_save_game))))
    (:then_1
      (for _index_2 (range 0 5)
        (CallFunction|AddBuildings)))))

(event EventTick
  (params (DeltaSeconds :type Float%20%28single-precision%29)))

(fn ConstructionScript)

(fn AddFloor
  (bind _returnvalue (Game|SpawnActorfromClass "/Game/runner/blueprints/Florik.Florik_C" (Variables|Default|GetFloorAttachPoint) "Undefined" "MultiplyWithRoot" 0 0))
  (bind _returnvalue_2 (Default|GetAttachPoint _returnvalue))
  (Variables|Default|SetFloorAttachPoint _returnvalue_2)
  (Utilities|Array|Add (Variables|Default|GetFloor%20Tyles) _returnvalue)
  (bind _result (Math|Integer|IncrementInt (Variables|Default|GetFloor%20Count))
    (:%20%20
      (Variables|Default|SetFloor%20Count _result))))

(fn ExtendFloor
  (bind _floor_tyles (Variables|Default|GetFloor%20Tyles))
  (bind _output (Utilities|Array|Get(acopy) _floor_tyles))
  (CallFunction|AddFloor)
  (if (> (Utilities|Array|Length (Variables|Default|GetFloor%20Tyles)) (+ (Variables|Default|GetNumber%20of%20Tyles) 11))
    (Actor|DestroyActor _output)
    (Utilities|Array|RemoveItem _floor_tyles _output)))

(fn AddBuildings
  (bind _returnvalue (Game|SpawnActorfromClass "/Game/runner/blueprints/Buildings.Buildings_C" (Variables|Default|GetBuilding%20SP) "Undefined" "MultiplyWithRoot" 0 0))
  (bind _returnvalue_2 (Default|GetAttachPoint _returnvalue))
  (Variables|Default|SetBuilding%20SP _returnvalue_2)
  (Utilities|Array|Add (Variables|Default|GetBuildings) _returnvalue))

(fn ExtendBuildings
  (bind _buildings (Variables|Default|GetBuildings))
  (bind _output (Utilities|Array|Get(acopy) _buildings))
  (CallFunction|AddBuildings)
  (if (> (Utilities|Array|Length (Variables|Default|GetBuildings)) 8)
    (Actor|DestroyActor _output)
    (Utilities|Array|RemoveItem _buildings _output)))