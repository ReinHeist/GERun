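; ObstaclesBlocker is a runner obstacle that the player must slide under to survive.
; On actor overlap it casts the other actor to run_character and checks its Issliding flag.
; If the character is not sliding, it calls Death, waits one second, then pauses the game.
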(event EventBeginPlay
  (|CallParentFunction) ; This node is disabled and will not be called.\nDrag off pins to build functionality.
)

(event Collision|EventActorBeginOverlap
  (params (OtherActor :type Actor%20Object%20Reference))
  (bind _asrun_character (Utilities|Casting|CastTorun_character OtherActor))
  (if (not (Variables|/Game/runner/blueprints/run_character.run_character_C|Getissliding _asrun_character))
    (Default|Death _asrun_character)
    (Utilities|FlowControl|Delay 1.0)
    (Game|SetGamePaused true)))

(event EventTick
  (params (DeltaSeconds :type Float%20%28single-precision%29))
  (|CallParentFunction DeltaSeconds) ; This node is disabled and will not be called.\nDrag off pins to build functionality.
)

(fn ConstructionScript
  (|CallParentFunction))